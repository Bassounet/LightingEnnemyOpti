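; BP_MenToDetect is a detection target that holds twelve zones named as light-scoring zones.
; On BeginPlay it gathers the W through W11 references into the ZoneScoringLight array and stores the count in HowManyZone.
; The Lighted? event only records the SphereCollided it receives in ZoneScoringLight0.
; No scoring or light test happens in this Blueprint, and the construction script is empty.
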(event EventLighted?
  (params (SphereCollided :type Array%20of%20Sphere%20Component%20Object%20References))
  (Variables|Default|SetZoneScoringLight_0 SphereCollided))

(event EventBeginPlay
  (bind _w10 (Variables|Default|Getw10))
  (bind _w9 (Variables|Default|Getw9))
  (bind _w8 (Variables|Default|Getw8))
  (bind _w7 (Variables|Default|Getw7))
  (bind _w6 (Variables|Default|Getw6))
  (bind _w11 (Variables|Default|Getw11))
  (bind _w3 (Variables|Default|Getw3))
  (bind _w4 (Variables|Default|Getw4))
  (bind _w2 (Variables|Default|Getw2))
  (bind _w1 (Variables|Default|Getw1))
  (bind _w (Variables|Default|Getw))
  (bind _w5 (Variables|Default|Getw5))
  (bind _array (Utilities|Array|MakeArray _w5 _w10 _w9 _w8 _w7 _w6 _w11 _w3 _w4 _w2 _w1 _w))
  (Variables|Default|SetZoneScoringLight _array)
  (Variables|Default|SetHowManyZone? (Utilities|Array|Length _array)))

(fn ConstructionScript)